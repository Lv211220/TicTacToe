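; Tic-tac-toe game mode that runs the match flow for two-player or player-versus-robot play.
; PrePlay initializes the game, shows the Start widget and cursor, and clears state; restart reruns it and rebinds the cell handler.
; Each cell change is checked for win, no moves or next turn, raising GameOver (always passing Player1) or toggling players after a short delay.
; After human turns, RobotStep fires the robot's move through the same cell-change event.
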(event `self.ReceiveBeginPlay`
  (`self.PrePlay`)
  (add `self.GameOver` (delegate `CustomEvent_0`))
  (add `self.OnCellStateChanged` (delegate `CellStateChanged_Event`))
  (add `self.GameRestart` (delegate `RestartGame`)))

(event `CustomEvent_0` :!signature `self.GameOver`
  (params (Player :type "ETurnState Enum" :default "Player1") (Result :type "EResultState Enum" :default "Win"))
  (set `self.Running` false)
  (set `self.Result` Result))

(event `RestartGame`
  (`self.PrePlay`)
  (add `self.OnCellStateChanged` (delegate `CellStateChanged_Event`)))

(event `RobotStep`
  (params (DefaultNum :type Integer))
  (bind _returnvalue (`self.GetRobotNum` DefaultNum))
  (`self.OnCellStateChanged` _returnvalue))

(event `CellStateChanged_Event`
  (params (Id :type Integer))
  (bind _returnvalue (`self.GetCurrentPlayer`))
  (if (`self.IsRobotMode`)
    ;[1 1 1] 人机对战
    (if (`|EnumEquality` "Player2" _returnvalue)
      (switch `EResultState` (`self.CheckRobotResult` Id)
        (:`Win`
          (`self.GameOver` "Player1" "Win"))
        (:`NoMore`
          (`self.GameOver` "Player1" "NoMore"))
        (:`PlayerNext`
          (`KismetSystemLibrary.Delay` 0.1)
          (`self.TogglePlayer` (`KismetMathLibrary.Conv_IntToBool` (`KismetMathLibrary.Conv_ByteToInt` _returnvalue)))))
      (else
        (switch `EResultState` (`self.CheckPlayerResult` Id)
          (:`Win`
            (`self.GameOver` "Player1" "Win"))
          (:`NoMore`
            (`self.GameOver` "Player1" "NoMore"))
          (:`PlayerNext`
            (`KismetSystemLibrary.Delay` 0.1)
            (`self.TogglePlayer` (`KismetMathLibrary.Conv_IntToBool` (`KismetMathLibrary.Conv_ByteToInt` _returnvalue)))
            (`self.RobotStep` -1)))))
    (else
      ;[1 1 1] 人人对战
      (bind _returnvalue_2 (`self.PlayerPlay` Id))
      (switch `EResultState` _returnvalue_2
        (:`Win`
          (`self.GameOver` "Player1" "Win"))
        (:`NoMore`
          (`self.GameOver` "Player1" "NoMore"))
        (:`PlayerNext`
          (`KismetSystemLibrary.Delay` 0.1)
          (`self.TogglePlayer` (`KismetMathLibrary.Conv_IntToBool` (`KismetMathLibrary.Conv_ByteToInt` (`self.GetCurrentPlayer`)))))))))

(fn `PrePlay`
  (bind _returnvalue (`GameplayStatics.GetPlayerControllerFromID` 0))
  (`self.GameInit`)
  (clear `self.OnCellStateChanged`)
  (bind _returnvalue_2 (`|CreateWidget` "/Game/UI/Start.Start_C" _returnvalue))
  (`UserWidget.AddToViewport` _returnvalue_2 0)
  (set `PlayerController.bShowMouseCursor` true _returnvalue)
  (set `self.Running` true)
  (set `self.History1` "")
  (set `self.History2` ""))

(fn `UserConstructionScript`)